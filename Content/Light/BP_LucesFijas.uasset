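; Fixed light actor with two spot-and-point style sets of light components and a Base mesh, apparently left over from a flicker setup.
; On Tick, a DoOnce gate waits a short randomized delay, then toggles the visibility of three spot lights and one point light.
; A FlipFlop that would set the Base material and reset the gate is disconnected, so the toggle happens only once.
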(event `self.ReceiveTick`
  (params (DeltaSeconds :type "Float (single-precision)"))
  (`/Engine/EditorBlueprintResources/StandardMacros.DoOnce` false
    (:`Completed`
      (`KismetSystemLibrary.RetriggerableDelay` (`KismetMathLibrary.RandomFloatInRange` (`KismetMathLibrary.RandomFloatInRange` 0.1 0.2) (`KismetMathLibrary.RandomFloatInRange` 0.4 0.5)))
      (`SceneComponent.ToggleVisibility` (`self.SpotLight`) false)
      (`SceneComponent.ToggleVisibility` (`self.PointLight`) false)
      (`SceneComponent.ToggleVisibility` (`self.SpotLight1`) false)
      (`SceneComponent.ToggleVisibility` (`self.SpotLight2`) false))))

(fn `UserConstructionScript`)