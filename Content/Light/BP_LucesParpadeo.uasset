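; Flickering light actor that blinks a SpotLight and a PointLight at irregular intervals.
; Tick runs through a DoOnce into a retriggerable delay with a nested random duration, then toggles both lights' visibility.
; A FlipFlop sets the first material slot of Luz on each toggle and resets the DoOnce, so the cycle repeats indefinitely.
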(event `self.ReceiveTick`
  (params (DeltaSeconds :type "Float (single-precision)"))
  (bind _luz (`self.Luz`))
  (`/Engine/EditorBlueprintResources/StandardMacros.DoOnce` false :!label _label
    (:`Completed`
      (`KismetSystemLibrary.RetriggerableDelay` (`KismetMathLibrary.RandomFloatInRange` (`KismetMathLibrary.RandomFloatInRange` 0.1 0.2) (`KismetMathLibrary.RandomFloatInRange` 0.4 0.5)))
      (`SceneComponent.ToggleVisibility` (`self.SpotLight`) false)
      (`SceneComponent.ToggleVisibility` (`self.PointLight`) false)
      (`/Engine/EditorBlueprintResources/StandardMacros.FlipFlop`
        (:`A`
          (`PrimitiveComponent.SetMaterial` _luz 0 null)
          (goto _label :!via `Reset`))
        (:`B`
          (`PrimitiveComponent.SetMaterial` _luz 0 null)
          (goto _label :!via `Reset`))))))

(fn `UserConstructionScript`)