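; BP_Button is a puzzle button that opens every BP_DoorButton whose DoorNum matches its ButtonNum on Interaction.
; From BeginPlay it blinks two lights in an endless Delay loop and adds an audio component.
; Interaction also plays the AnimButton timeline to move the button mesh, then after a short delay destroys the lights and audio and reverses the timeline.
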(event `self.ReceiveBeginPlay`
  (`|ExecutionSequence`
    (:`then_0`
      (`SceneComponent.SetVisibility` (`self.Luz1`) (`self.Luces`) false :!label _label)
      (`SceneComponent.SetVisibility` (`self.Luz2`) (`self.Luces`) false)
      (`KismetSystemLibrary.Delay` 0.4)
      (`SceneComponent.SetVisibility` (`self.Luz2`) (`self.NoLuz`) true)
      (`SceneComponent.SetVisibility` (`self.Luz1`) (`self.NoLuz`) true)
      (`KismetSystemLibrary.Delay` 0.4)
      (goto _label))
    (:`then_1`
      (bind _returnvalue (`AddComponent|NODE_AddAudioComponent-3`)))))

(event `/Game/Puzzle/ButtonPuzzle/BPI_Interaction.Interaction`
  (params (RefJugador :type "/Game/FirstPerson/Blueprints/BP_FirstPersonCharacter Object Reference"))
  (`|ExecutionSequence`
    (:`then_0`
      (bind _outactors (`GameplayStatics.GetAllActorsOfClass` "/Game/Puzzle/ButtonPuzzle/BP_DoorButton.BP_DoorButton_C"))
      (for _array_element _outactors
        (if (== (`/Game/Puzzle/ButtonPuzzle/BP_DoorButton.DoorNum` _array_element) (`self.ButtonNum`))
          (`/Game/Puzzle/ButtonPuzzle/BP_DoorButton.OpenDoor` _array_element))))
    (:`then_1`
      (bind (_direction _newtrack_0) (`Timeline|AnimButton` :!label _label_2)
        (:`Update`
          (`SceneComponent.K2_SetRelativeLocation` (`self.Button`) (`KismetMathLibrary.MakeVector` _newtrack_0) false false)
          (`KismetSystemLibrary.Delay` 0.1)
          (`ActorComponent.K2_DestroyComponent` (`self.Luz1`))
          (`ActorComponent.K2_DestroyComponent` (`self.Luz2`))
          (`ActorComponent.K2_DestroyComponent` (stale `self.ReceiveBeginPlay` _returnvalue))
          (goto _label_2 :!via `Reverse`))))))

(fn `UserConstructionScript`)