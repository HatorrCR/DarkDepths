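; Direction puzzle actor with two statues that the player rotates until both activate.
; Each statue's player trigger enables input and opens a gate, letting IA_Interact turn it by AngleRotation through a timeline lerp, with input locked mid-turn.
; Puzzle triggers flag each statue active while overlapping a BP_ActivadorEstatuas.
; A looping timer polls both flags and calls PuzzleResuelto when both are set.
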(event `PuzzleResuelto`
  ;[0 0 0] Inicio y Soluci'on
  (if (and (`self.Estatua1Activada?`) (`self.Estatua2Activada?`))
    (`self.PuzzleResuelto`)))

(event `self.ReceiveBeginPlay`
  ;[0 0 0] Inicio y Soluci'on
  (`|ExecutionSequence`
    (:`then_0`
      (set `self.CurrentRotationEstatua1` (`SceneComponent.K2_GetComponentRotation` (`self.Estatua_1`)))
      (set `self.CurrentRotationEstatua2` (`SceneComponent.K2_GetComponentRotation` (`self.Estatua_2`))))
    (:`then_1`
      (`KismetSystemLibrary.K2_SetTimer` null "PuzzleResuelto" 0.25 true))))

(event `EnhancedInput|/Game/FirstPerson/Input/Actions/IA_Interact`
  (params (ActionValue :type Boolean) (ElapsedSeconds :type "Float (double-precision)") (TriggeredSeconds :type "Float (double-precision)") (InputAction :type "InputAction Object Reference" :default "/Game/FirstPerson/Input/Actions/IA_Interact.IA_Interact"))
  ;[0 0 0] Estatua1
  (:`Triggered`
    (`/Engine/EditorBlueprintResources/StandardMacros.Gate` true :!label _label
      (:`Exit`
        (`self.DisableInput` (`GameplayStatics.GetPlayerController` 0))
        (bind (_direction _timeline_statua) (`Timeline|Timeline Estatua1` :!via `PlayFromStart`)
          (:`Update`
            (bind _returnvalue (`KismetMathLibrary.RLerp` (`self.CurrentRotationEstatua1`) (`KismetMathLibrary.MakeRotator` (.roll (`self.CurrentRotationEstatua1`)) (.pitch (`self.CurrentRotationEstatua1`)) (+ (.yaw (`self.CurrentRotationEstatua1`)) (`self.AngleRotation`))) _timeline_statua))
            (`SceneComponent.K2_SetRelativeRotation` (`self.Estatua_1`) _returnvalue false false))
          (:`Finished`
            (set `self.CurrentRotationEstatua1` _returnvalue)
            (`self.EnableInput` (`GameplayStatics.GetPlayerController` 0))))))))

(event `self.TriggerActivadorStatua1.OnComponentBeginOverlap`
  (params (OverlappedComponent :type "PrimitiveComponent Object Reference") (OtherActor :type "Actor Object Reference") (OtherComp :type "PrimitiveComponent Object Reference") (OtherBodyIndex :type Integer) (bFromSweep :type Boolean) (SweepResult :type "HitResult Structure (by ref)"))
  ;[0 0 0] Estatua1
  (cast `/Game/FirstPerson/Blueprints/BP_FirstPersonCharacter` OtherActor)
  (`self.EnableInput` (`GameplayStatics.GetPlayerController` 0))
  (goto _label :!via `Open`))

(event `self.TriggerActivadorStatua1.OnComponentEndOverlap`
  (params (OverlappedComponent :type "PrimitiveComponent Object Reference") (OtherActor :type "Actor Object Reference") (OtherComp :type "PrimitiveComponent Object Reference") (OtherBodyIndex :type Integer))
  ;[0 0 0] Estatua1
  (cast `/Game/FirstPerson/Blueprints/BP_FirstPersonCharacter` OtherActor)
  (`self.DisableInput` (`GameplayStatics.GetPlayerController` 0))
  (goto _label :!via `Close`))

(event `self.TriggerActivadorPuzzle1.OnComponentBeginOverlap`
  (params (OverlappedComponent :type "PrimitiveComponent Object Reference") (OtherActor :type "Actor Object Reference") (OtherComp :type "PrimitiveComponent Object Reference") (OtherBodyIndex :type Integer) (bFromSweep :type Boolean) (SweepResult :type "HitResult Structure (by ref)"))
  ;[0 0 0] Estatua1
  (cast `/Game/Puzzle/DirectionPuzzle/BP_ActivadorEstatuas` OtherActor)
  (set `self.Estatua1Activada?` true))

(event `self.TriggerActivadorPuzzle1.OnComponentEndOverlap`
  (params (OverlappedComponent :type "PrimitiveComponent Object Reference") (OtherActor :type "Actor Object Reference") (OtherComp :type "PrimitiveComponent Object Reference") (OtherBodyIndex :type Integer))
  ;[0 0 0] Estatua1
  (cast `/Game/Puzzle/DirectionPuzzle/BP_ActivadorEstatuas` OtherActor)
  (set `self.Estatua1Activada?` false))

(event `EnhancedInput|/Game/FirstPerson/Input/Actions/IA_Interact`
  (params (ActionValue :type Boolean) (ElapsedSeconds :type "Float (double-precision)") (TriggeredSeconds :type "Float (double-precision)") (InputAction :type "InputAction Object Reference" :default "/Game/FirstPerson/Input/Actions/IA_Interact.IA_Interact"))
  ;[0 0 0] Comment
  (:`Triggered`
    (`/Engine/EditorBlueprintResources/StandardMacros.Gate` true :!label _label_2
      (:`Exit`
        (`self.DisableInput` (`GameplayStatics.GetPlayerController` 0))
        (bind (_direction _timeline_statua) (`Timeline|Timeline` :!via `PlayFromStart`)
          (:`Update`
            (bind _returnvalue (`KismetMathLibrary.RLerp` (`self.CurrentRotationEstatua2`) (`KismetMathLibrary.MakeRotator` (.roll (`self.CurrentRotationEstatua2`)) (.pitch (`self.CurrentRotationEstatua2`)) (+ (.yaw (`self.CurrentRotationEstatua2`)) (`self.AngleRotation`))) _timeline_statua))
            (`SceneComponent.K2_SetRelativeRotation` (`self.Estatua_2`) _returnvalue false false))
          (:`Finished`
            (set `self.CurrentRotationEstatua2` _returnvalue)
            (`self.EnableInput` (`GameplayStatics.GetPlayerController` 0))))))))

(event `self.TriggerActivadorStatua2.OnComponentBeginOverlap`
  (params (OverlappedComponent :type "PrimitiveComponent Object Reference") (OtherActor :type "Actor Object Reference") (OtherComp :type "PrimitiveComponent Object Reference") (OtherBodyIndex :type Integer) (bFromSweep :type Boolean) (SweepResult :type "HitResult Structure (by ref)"))
  ;[0 0 0] Comment
  (cast `/Game/FirstPerson/Blueprints/BP_FirstPersonCharacter` OtherActor)
  (`self.EnableInput` (`GameplayStatics.GetPlayerController` 0))
  (goto _label_2 :!via `Open`))

(event `self.TriggerActivadorStatua2.OnComponentEndOverlap`
  (params (OverlappedComponent :type "PrimitiveComponent Object Reference") (OtherActor :type "Actor Object Reference") (OtherComp :type "PrimitiveComponent Object Reference") (OtherBodyIndex :type Integer))
  ;[0 0 0] Comment
  (cast `/Game/FirstPerson/Blueprints/BP_FirstPersonCharacter` OtherActor)
  (`self.DisableInput` (`GameplayStatics.GetPlayerController` 0))
  (goto _label_2 :!via `Close`))

(event `self.TriggerActivadorPuzzle2.OnComponentBeginOverlap`
  (params (OverlappedComponent :type "PrimitiveComponent Object Reference") (OtherActor :type "Actor Object Reference") (OtherComp :type "PrimitiveComponent Object Reference") (OtherBodyIndex :type Integer) (bFromSweep :type Boolean) (SweepResult :type "HitResult Structure (by ref)"))
  ;[0 0 0] Comment
  (cast `/Game/Puzzle/DirectionPuzzle/BP_ActivadorEstatuas` OtherActor)
  (set `self.Estatua2Activada?` true))

(event `self.TriggerActivadorPuzzle2.OnComponentEndOverlap`
  (params (OverlappedComponent :type "PrimitiveComponent Object Reference") (OtherActor :type "Actor Object Reference") (OtherComp :type "PrimitiveComponent Object Reference") (OtherBodyIndex :type Integer))
  ;[0 0 0] Comment
  (cast `/Game/Puzzle/DirectionPuzzle/BP_ActivadorEstatuas` OtherActor)
  (set `self.Estatua2Activada?` false))

(fn `UserConstructionScript`)