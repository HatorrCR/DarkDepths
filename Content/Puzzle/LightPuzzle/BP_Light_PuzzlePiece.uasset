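; Light puzzle piece Blueprint that cycles its point light through five preset colors when used.
; OnUse waits briefly, increments ColorIndex and wraps it back to zero after the last color.
; UpdateLightColor then switches on the index to set the PointLight to white, green, red, yellow or light blue.
; The file holds no solution check, only the color cycling.
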(event `/Game/Puzzle/LightPuzzle/BPI_UseInterface.OnUse`
  (params (Actor :type "Actor Object Reference"))
  (`KismetSystemLibrary.Delay` 0.2)
  (bind _result (`/Engine/EditorBlueprintResources/StandardMacros.IncrementInt` (`self.ColorIndex`))
    (:`  `
      (if (not (<= _result 4))
        (set `self.ColorIndex` 0))
      (`self.UpdateLightColor`))))

(fn `UpdateLightColor`
  (switch `int` (`self.ColorIndex`)
    (:`0`
      (`LightComponent.SetLightColor` (`self.PointLight`) (struct :`R` 1.0 :`G` 1.0 :`B` 1.0 :`A` 1.0) true))
    (:`1`
      (`LightComponent.SetLightColor` (`self.PointLight`) (struct :`R` 0.036388 :`G` 0.858001 :`A` 1.0) true))
    (:`2`
      (`LightComponent.SetLightColor` (`self.PointLight`) (struct :`R` 0.776 :`A` 1.0) true))
    (:`3`
      (`LightComponent.SetLightColor` (`self.PointLight`) (struct :`R` 0.91 :`G` 0.710548 :`A` 1.0) true))
    (:`4`
      (`LightComponent.SetLightColor` (`self.PointLight`) (struct :`R` 0.08 :`G` 0.705498 :`B` 1.0 :`A` 1.0) true))))

(fn `UserConstructionScript`)