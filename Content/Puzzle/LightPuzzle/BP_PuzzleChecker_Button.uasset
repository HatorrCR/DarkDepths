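; Button actor for a light puzzle that checks the piece colours when used and triggers a door if they match.
; Each entry in PuzzlePieces has its ColorIndex compared against ColorCode at the same array position.
; A match sends OnUseMessage once to DoorToOpen through BPI_UseInterface, while a mismatch resets every piece to colour zero and refreshes its light.
; A Timeline for moving the button's Cube is present but never runs.
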(event `/Game/Puzzle/LightPuzzle/BPI_UseInterface.OnUse`
  (params (Actor :type "Actor Object Reference"))
  (set `self.IsCorrect` true)
  (for (_array_element _array_index) (`self.PuzzlePieces`)
    (if (!= (`/Game/Puzzle/LightPuzzle/BP_Light_PuzzlePiece.ColorIndex` _array_element) (`|GetArrayItem` (`self.ColorCode`) _array_index))
      (set `self.IsCorrect` false)
      (break)))
  (if (`self.IsCorrect`)
    (`/Engine/EditorBlueprintResources/StandardMacros.DoOnce` false
      (:`Completed`
        (bind _doortoopen (`self.DoorToOpen`)
          (:`then`
            (`|ExecutionSequence`
              (:`then_1`
                (if (`KismetSystemLibrary.DoesImplementInterface` _doortoopen "/Game/Puzzle/LightPuzzle/BPI_UseInterface.BPI_UseInterface_C")
                  (message `/Game/Puzzle/LightPuzzle/BPI_UseInterface.OnUse` _doortoopen self)))))
          (:`else`))))
    (else
      (for _array_element_2 (`self.PuzzlePieces`)
        (set `/Game/Puzzle/LightPuzzle/BP_Light_PuzzlePiece.ColorIndex` 0 _array_element_2)
        (`/Game/Puzzle/LightPuzzle/BP_Light_PuzzlePiece.UpdateLightColor` _array_element_2)))))

(fn `UserConstructionScript`)