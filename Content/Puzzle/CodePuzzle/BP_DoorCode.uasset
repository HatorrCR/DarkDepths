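; Keypad-code puzzle door whose mesh and material are set in the construction script.
; Overlapping Box3 as the first-person character shows the prompt and enables input, so IA_Codigo toggles the WI_DoorCode widget with mouse cursor.
; OpenDoorCode, not called within this Blueprint, swings the door's yaw by Angle through the Door_Slide timeline.
; A delay started from the timeline's Update reverses it after five seconds.
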(event `OpenDoorCode`
  (bind (_direction _newtrack_0) (`Timeline|Door_Slide` :!label _label)
    (:`Update`
      (`SceneComponent.K2_SetRelativeRotation` (`self.Door`) (`KismetMathLibrary.MakeRotator` 0.0 0.0 (* _newtrack_0 (`self.Angle`))) false false)
      (`KismetSystemLibrary.Delay` 5.0)
      (goto _label :!via `Reverse`))))

(event `EnhancedInput|/Game/FirstPerson/Input/Actions/IA_Codigo`
  (params (ActionValue :type Boolean) (ElapsedSeconds :type "Float (double-precision)") (TriggeredSeconds :type "Float (double-precision)") (InputAction :type "InputAction Object Reference" :default "/Game/FirstPerson/Input/Actions/IA_Codigo.IA_Codigo"))
  (bind _returnvalue (`GameplayStatics.GetPlayerController` 0))
  (:`Completed`
    (`/Engine/EditorBlueprintResources/StandardMacros.FlipFlop`
      (:`A`
        (bind _returnvalue_2 (`|CreateWidget` "/Game/Puzzle/CodePuzzle/WI_DoorCode.WI_DoorCode_C"))
        (`UserWidget.AddToViewport` _returnvalue_2 0)
        (`WidgetBlueprintLibrary.SetInputMode_GameAndUIEx` _returnvalue _returnvalue_2)
        (set `PlayerController.bShowMouseCursor` true _returnvalue))
      (:`B`
        (`WidgetLayoutLibrary.RemoveAllWidgets`)
        (`WidgetBlueprintLibrary.SetInputMode_GameOnly` _returnvalue)
        (set `PlayerController.bShowMouseCursor` false _returnvalue)))))

(event `self.Box3.OnComponentBeginOverlap`
  (params (OverlappedComponent :type "PrimitiveComponent Object Reference") (OtherActor :type "Actor Object Reference") (OtherComp :type "PrimitiveComponent Object Reference") (OtherBodyIndex :type Integer) (bFromSweep :type Boolean) (SweepResult :type "HitResult Structure (by ref)"))
  (cast `/Game/FirstPerson/Blueprints/BP_FirstPersonCharacter` OtherActor)
  (`self.EnableInput` (`GameplayStatics.GetPlayerController` 0))
  (`SceneComponent.SetVisibility` (`self.Texto`) true false))

(event `self.Box3.OnComponentEndOverlap`
  (params (OverlappedComponent :type "PrimitiveComponent Object Reference") (OtherActor :type "Actor Object Reference") (OtherComp :type "PrimitiveComponent Object Reference") (OtherBodyIndex :type Integer))
  (cast `/Game/FirstPerson/Blueprints/BP_FirstPersonCharacter` OtherActor)
  (`self.DisableInput` (`GameplayStatics.GetPlayerController` 0))
  (`SceneComponent.SetVisibility` (`self.Texto`) false false))

(fn `UserConstructionScript`
  (bind _door (`self.Door`))
  (`PrimitiveComponent.SetCollisionEnabled` _door "QueryOnly")
  (`StaticMeshComponent.SetStaticMesh` _door (`self.Static Mesh`))
  (`PrimitiveComponent.SetMaterial` _door 0 (`self.Material`)))